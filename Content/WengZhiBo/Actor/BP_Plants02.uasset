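; BP_Plants02 is an actor, by its name a plant, that scales up from nothing while its point light fades in.
; BeginPlay hides it by zeroing the Scene1 scale and light intensity.
; Tick polls the ScaleLight flag, which is set outside this graph, then uses DoOnce to play a timeline driving both scale and intensity.
; The construction script applies configurable intensity, source radius and attenuation radius to the light.
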(event `self.ReceiveBeginPlay`
  (`SceneComponent.SetRelativeScale3D` (`self.Scene1`) (0.0 0.0 0.0))
  (`LightComponent.SetIntensity` (`self.PointLight`) 0.0))

(event `self.ReceiveTick`
  (params (DeltaSeconds :type "Float (single-precision)"))
  (if (`self.Scale_Light`)
    (`/Engine/EditorBlueprintResources/StandardMacros.DoOnce` false
      (:`Completed`
        (bind (_direction `_新建轨道_0`) (`Timeline|时间轴_0` :!via `PlayFromStart`)
          (:`Update`
            (bind _returnvalue (`KismetMathLibrary.Lerp` 0.0 1.0 `_新建轨道_0`))
            (`SceneComponent.SetRelativeScale3D` (`self.Scene1`) (`KismetMathLibrary.Conv_DoubleToVector` _returnvalue))
            (`LightComponent.SetIntensity` (`self.PointLight`) (`KismetMathLibrary.Lerp` 0.0 (`self.强度`) _returnvalue))))))))

(fn `UserConstructionScript`
  (bind _pointlight (`self.PointLight`))
  (`LightComponent.SetIntensity` _pointlight (`self.强度`))
  (`PointLightComponent.SetSourceRadius` _pointlight (`self.源半径`))
  (`LocalLightComponent.SetAttenuationRadius` _pointlight (`self.衰减半径`)))