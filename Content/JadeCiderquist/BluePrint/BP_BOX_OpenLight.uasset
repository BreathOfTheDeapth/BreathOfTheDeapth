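; Trigger box that lights up an area once when the VR player pawn enters it.
; BeginPlay sets every spotlight in its array to zero intensity.
; The first overlap sets the ScaleLight flag on two plant arrays (mushrooms), then steps through the spotlights with a delayed loop.
; Each step restarts one shared timeline that lerps the current light from zero up to a target intensity, so lights brighten in sequence.
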(event `self.ReceiveBeginPlay`
  (bind _spot_light (`self.Spot_Light`))
  ;[1 1 1] 开始运行灯光关闭
  (bind (_array_element _array_index) (`/Game/AFCore/Libraries/MLib_Actor_Macros.ForEachLoopWithDelay` _spot_light)
    (:`LoopBody`
      (`LightComponent.SetIntensity` (`Light.LightComponent` (`|GetArrayItem` _spot_light _array_index)) 0.0))))

(event `self.Box.OnComponentBeginOverlap`
  (params (OverlappedComponent :type "PrimitiveComponent Object Reference") (OtherActor :type "Actor Object Reference") (OtherComp :type "PrimitiveComponent Object Reference") (OtherBodyIndex :type Integer) (bFromSweep :type Boolean) (SweepResult :type "HitResult Structure (by ref)"))
  (bind _plants01 (`self.Plants01`))
  (bind _plants02 (`self.Plants02`))
  (bind _spot_light (`self.Spot_Light`))
  (cast `/Game/AFCore/Examples/Pawns/VR/BP_Pawn_VR_Char_Example_HandsOn` OtherActor)
  (`/Engine/EditorBlueprintResources/StandardMacros.DoOnce` false
    (:`Completed`
      ;[1 1 1] 蘑菇
      (for (_ _array_index) _plants01
        (set `/Game/WengZhiBo/Actor/BP_Plants01.Scale_Light` true (`|GetArrayItem` _plants01 _array_index)))
      (for (_ _array_index_2) _plants02
        (set `/Game/WengZhiBo/Actor/BP_Plants02.Scale_Light` true (`|GetArrayItem` _plants02 _array_index_2)))
      ;[1 1 1] 灯光变亮
      (bind (_array_element _array_index_3) (`/Game/AFCore/Libraries/MLib_Actor_Macros.ForEachLoopWithDelay` _spot_light 3.0)
        (:`LoopBody`
          (bind (_direction `_新建轨道_0`) (`Timeline|时间轴_0` :!via `PlayFromStart`)
            (:`Update`
              (`LightComponent.SetIntensity` (`Light.LightComponent` (`|GetArrayItem` _spot_light _array_index_3)) (`KismetMathLibrary.Lerp` 0.0 (`self.灯光强度`) `_新建轨道_0`)))))))))

(fn `UserConstructionScript`)