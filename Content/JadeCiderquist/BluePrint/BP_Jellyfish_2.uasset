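; BP_Jellyfish_2 is a glowing jellyfish checkpoint in a VR movement tutorial, triggered when the player pawn overlaps its sphere.
; The construction script applies materials, tints the point light from Glow_Color and sets whether overlap starts enabled.
; Number selects the step: early steps swap direction prompts with audio and activate the next tagged jellyfish.
; The final step shows success, freezes the pawn, fades MP_UnderWater light out, teleports it, fades in and triggers BP_Title.
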(event `self.ReceiveTick`
  (params (DeltaSeconds :type "Float (single-precision)")))

(event `self.Sphere.OnComponentBeginOverlap`
  (params (OverlappedComponent :type "PrimitiveComponent Object Reference") (OtherActor :type "Actor Object Reference") (OtherComp :type "PrimitiveComponent Object Reference") (OtherBodyIndex :type Integer) (bFromSweep :type Boolean) (SweepResult :type "HitResult Structure (by ref)"))
  (bind _asbp_pawn_vr_char_example_hands_on (cast `/Game/AFCore/Examples/Pawns/VR/BP_Pawn_VR_Char_Example_HandsOn` OtherActor))
  (set `/Game/AFCore/Examples/Pawns/VR/BP_Pawn_VR_Char_Example_HandsOn.if_Prompt` false _asbp_pawn_vr_char_example_hands_on)
  (switch `int` (`self.Number`)
    (:`0`
      ;[1 1 1] Forward
      (bind _outactors (`GameplayStatics.GetAllActorsOfClass` "/Game/JadeCiderquist/Widget/WBP_Forward.WBP_Forward_C"))
      (`self.SetActorHiddenInGame` (`|GetArrayItem` _outactors) true)
      (bind _outactors_2 (`GameplayStatics.GetAllActorsOfClass` "/Game/JadeCiderquist/Widget/WBP_Left.WBP_Left_C"))
      (bind _output (`|GetArrayItem` _outactors_2))
      (`self.SetActorHiddenInGame` _output false)
      (`AudioComponent.Play` (`/Game/JadeCiderquist/Widget/WBP_Left.Audio` _output) 0.0)
      (bind _outactors_3 (`GameplayStatics.GetAllActorsOfClassWithTag` "BP_Jellyfish_2_C" "Jellyfish1"))
      (bind _output_2 (`|GetArrayItem` _outactors_3))
      (`self.SetActorHiddenInGame` _output_2 false)
      (set `PrimitiveComponent.bGenerateOverlapEvents` true (`/Game/JadeCiderquist/BluePrint/BP_Jellyfish_2.Sphere` _output_2))
      (`self.K2_DestroyActor`))
    (:`1`
      ;[1 1 1] Down
      (bind _outactors_4 (`GameplayStatics.GetAllActorsOfClass` "/Game/JadeCiderquist/Widget/WBP_Left.WBP_Left_C"))
      (`self.SetActorHiddenInGame` (`|GetArrayItem` _outactors_4) true)
      (`self.K2_DestroyActor`)
      (bind _outactors_5 (`GameplayStatics.GetAllActorsOfClass` "/Game/JadeCiderquist/Widget/WBP_Up.WBP_Up_C"))
      (bind _output_3 (`|GetArrayItem` _outactors_5))
      (`self.SetActorHiddenInGame` _output_3 false)
      (`AudioComponent.Play` (`/Game/JadeCiderquist/Widget/WBP_Up.Audio` _output_3) 0.0)
      (bind _outactors_6 (`GameplayStatics.GetAllActorsOfClassWithTag` "BP_Jellyfish_2_C" "Jellyfish2"))
      (bind _output_4 (`|GetArrayItem` _outactors_6))
      (`self.SetActorHiddenInGame` _output_4 false)
      (set `PrimitiveComponent.bGenerateOverlapEvents` true (`/Game/JadeCiderquist/BluePrint/BP_Jellyfish_2.Sphere` _output_4)))
    (:`2`
      ;[1 1 1] Top
      (bind _outactors_7 (`GameplayStatics.GetAllActorsOfClass` "/Game/JadeCiderquist/Widget/WBP_Up.WBP_Up_C"))
      (`self.SetActorHiddenInGame` (`|GetArrayItem` _outactors_7) true)
      (bind _outactors_8 (`GameplayStatics.GetAllActorsOfClassWithTag` "BP_Jellyfish_2_C" "Jellyfish2"))
      (bind _output_5 (`|GetArrayItem` _outactors_8))
      (`self.SetActorHiddenInGame` _output_5 true)
      (set `PrimitiveComponent.bGenerateOverlapEvents` false (`/Game/JadeCiderquist/BluePrint/BP_Jellyfish_2.Sphere` _output_5))
      (bind _outactors_9 (`GameplayStatics.GetAllActorsOfClass` "/Game/JadeCiderquist/Widget/WBP_MoveSucceed.WBP_MoveSucceed_C"))
      (bind _output_6 (`|GetArrayItem` _outactors_9))
      (`self.SetActorHiddenInGame` _output_6 false)
      (`AudioComponent.Play` (`/Game/JadeCiderquist/Widget/WBP_MoveSucceed.Audio` _output_6) 0.0)
      ;[1 1 1] 角色最后位置
      (bind _outactors_10 (`GameplayStatics.GetAllActorsOfClass` "/Game/AFCore/Examples/Pawns/VR/BP_Pawn_VR_Char_Example_HandsOn.BP_Pawn_VR_Char_Example_HandsOn_C"))
      (bind _output_7 (`|GetArrayItem` _outactors_10))
      (set `self.Final_Location` (`self.K2_GetActorLocation` _output_7))
      ;[1 1 1] 提升移动速度，禁止移动
      (set `/Game/AFCore/Examples/Pawns/VR/BP_Pawn_VR_Char_Example_HandsOn.Speed_Scale` 4.0 _output_7)
      (set `/Game/AFCore/Examples/Pawns/VR/BP_Pawn_VR_Char_Example_HandsOn.if_Move` false _output_7)
      (`KismetSystemLibrary.Delay` 2.0)
      ;[0 0 0] 渐渐变黑
      (bind (_direction `_新建轨道_0`) (`Timeline|时间轴_0` :!via `PlayFromStart`)
        (:`Update`
          (`KismetMaterialLibrary.SetScalarParameterValue` "/Game/JadeCiderquist/Material/Underwater/MP_UnderWater.MP_UnderWater" "Light" (`KismetMathLibrary.Lerp` 1.0 0.0 `_新建轨道_0`)))
        (:`Finished`
          ;[1 1 1] 角色坠落
          (set `/Game/AFCore/Examples/Pawns/VR/BP_Pawn_VR_Char_Example_HandsOn.if_Move` true _output_7)
          (`self.K2_SetActorLocation` _output_7 (`KismetMathLibrary.VLerp` (`self.Final_Location`) (2563.0 -943.0 1663.0) 1.0) false false)
          ;[0 0 0] 渐渐变亮
          (bind (_direction_2 `_新建轨道_0_2`) (`Timeline|时间轴_1` :!via `PlayFromStart`)
            (:`Update`
              (`KismetMaterialLibrary.SetScalarParameterValue` "/Game/JadeCiderquist/Material/Underwater/MP_UnderWater.MP_UnderWater" "Light" (`KismetMathLibrary.Lerp` 0.0 1.0 `_新建轨道_0_2`)))
            (:`Finished`
              ;[1 1 1] 播放标题
              (bind _outactors_11 (`GameplayStatics.GetAllActorsOfClass` "/Game/JadeCiderquist/Media/Title/BP_Title.BP_Title_C"))
              (set `/Game/JadeCiderquist/Media/Title/BP_Title.Play_Title` true (`|GetArrayItem` _outactors_11)))))))))

(fn `UserConstructionScript`
  (bind _sm_jellyfish0 (`self.SM_Jellyfish0`))
  (bind _returnvalue (`PrimitiveComponent.CreateDynamicMaterialInstance` _sm_jellyfish0 0 (`self.Material1`) "None"))
  (bind _returnvalue_2 (`MaterialInstanceDynamic.K2_GetVectorParameterValue` _returnvalue "Glow_Color"))
  (`LightComponent.SetLightColor` (`self.PointLight`) _returnvalue_2 true)
  (`PrimitiveComponent.SetMaterial` _sm_jellyfish0 0 _returnvalue)
  (`PrimitiveComponent.SetMaterial` _sm_jellyfish0 1 (`self.Material2`))
  (set `PrimitiveComponent.bGenerateOverlapEvents` (`self.Overlap`) (`self.Sphere`)))