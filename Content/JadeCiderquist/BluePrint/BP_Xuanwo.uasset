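; BP_Xuanwo is a spinning vortex (xuanwo) actor that reacts to touch by the VR player pawn.
; The construction script applies SourceMaterial to the mesh, BeginPlay stores a dynamic instance of it, and Tick rotates the mesh by a fixed, frame-dependent step.
; Mesh and capsule overlaps share one handler that prints a debug string and plays haptics on both hands.
; The level-opening node is disconnected, so no travel occurs.
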(event `self.ReceiveBeginPlay`
  (bind _returnvalue (`PrimitiveComponent.CreateDynamicMaterialInstance` (`self.M_XuanWo`) 0 (`self.Source Material`) "None"))
  (set `self.I_Material` _returnvalue))

(event `self.ReceiveTick`
  (params (DeltaSeconds :type "Float (single-precision)"))
  (`SceneComponent.K2_AddRelativeRotation` (`self.M_XuanWo`) (struct :`Yaw` -1.0) false false))

(event `self.M_XuanWo.OnComponentBeginOverlap`
  (params (OverlappedComponent :type "PrimitiveComponent Object Reference") (OtherActor :type "Actor Object Reference") (OtherComp :type "PrimitiveComponent Object Reference") (OtherBodyIndex :type Integer) (bFromSweep :type Boolean) (SweepResult :type "HitResult Structure (by ref)"))
  (bind _returnvalue (`GameplayStatics.GetPlayerController` 0))
  (cast `/Game/AFCore/Examples/Pawns/VR/BP_Pawn_VR_Char_Example_HandsOn` (stale `self.Capsule.OnComponentBeginOverlap` OtherActor) :!label _label)
  (`KismetSystemLibrary.PrintString` "Level")
  (`PlayerController.PlayHapticEffect` _returnvalue "/Game/JadeCiderquist/VRTemplate/Haptics/PistolFireHapticEffect.PistolFireHapticEffect" "Left" 1.0 false)
  (`PlayerController.PlayHapticEffect` _returnvalue "/Game/JadeCiderquist/VRTemplate/Haptics/PistolFireHapticEffect.PistolFireHapticEffect" "Right" 1.0 false))

(event `self.Capsule.OnComponentBeginOverlap`
  (params (OverlappedComponent :type "PrimitiveComponent Object Reference") (OtherActor :type "Actor Object Reference") (OtherComp :type "PrimitiveComponent Object Reference") (OtherBodyIndex :type Integer) (bFromSweep :type Boolean) (SweepResult :type "HitResult Structure (by ref)"))
  (goto _label))

(fn `UserConstructionScript`
  (`PrimitiveComponent.SetMaterial` (`self.M_XuanWo`) 0 (`self.Source Material`)))