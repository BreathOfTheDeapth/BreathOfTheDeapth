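; Black_Room is a VR room actor with destructible walls and a boundary that can send the player back to the start.
; When IfDes is true, Tick uses a DoOnce to enable physics simulation on six wall geometry collections.
; BeginPlay stores the location of the pawn tagged "Up_Hands".
; When the VR pawn leaves the Box, it returns to that location if the tagged BP_Jellyfish_2 has Restart set.
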(event `self.ReceiveTick`
  (params (DeltaSeconds :type "Float (single-precision)"))
  (if (`self.if_Des`)
    (`/Engine/EditorBlueprintResources/StandardMacros.DoOnce` false
      (:`Completed`
        (`PrimitiveComponent.SetSimulatePhysics` (`self.SM_Wall_GeometryCollection1`) true)
        (`PrimitiveComponent.SetSimulatePhysics` (`self.SM_Wall_GeometryCollection2`) true)
        (`PrimitiveComponent.SetSimulatePhysics` (`self.SM_Wall_GeometryCollection3`) true)
        (`PrimitiveComponent.SetSimulatePhysics` (`self.SM_Wall_GeometryCollection4`) true)
        (`PrimitiveComponent.SetSimulatePhysics` (`self.SM_Wall_GeometryCollection5`) true)
        (`PrimitiveComponent.SetSimulatePhysics` (`self.SM_Wall_GeometryCollection`) true)))))

(event `self.ReceiveBeginPlay`
  (bind _outactors (`GameplayStatics.GetAllActorsOfClassWithTag` "/Game/AFCore/Examples/Pawns/VR/BP_Pawn_VR_Char_Example_HandsOn.BP_Pawn_VR_Char_Example_HandsOn_C" "Up_Hands"))
  (set `self.Hands_Start` (`self.K2_GetActorLocation` (`|GetArrayItem` _outactors))))

(event `self.Box.OnComponentEndOverlap`
  (params (OverlappedComponent :type "PrimitiveComponent Object Reference") (OtherActor :type "Actor Object Reference") (OtherComp :type "PrimitiveComponent Object Reference") (OtherBodyIndex :type Integer))
  (bind _asbp_pawn_vr_char_example_hands_on (cast `/Game/AFCore/Examples/Pawns/VR/BP_Pawn_VR_Char_Example_HandsOn` OtherActor))
  (bind _outactors (`GameplayStatics.GetAllActorsOfClassWithTag` "/Game/JadeCiderquist/BluePrint/BP_Jellyfish_2.BP_Jellyfish_2_C" "Jellyfish2"))
  (if (`/Game/JadeCiderquist/BluePrint/BP_Jellyfish_2.Restart` (`|GetArrayItem` _outactors))
    (`self.K2_SetActorLocation` _asbp_pawn_vr_char_example_hands_on (`self.Hands_Start`) false false)))

(fn `UserConstructionScript`)