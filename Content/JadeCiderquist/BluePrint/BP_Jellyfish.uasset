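; Decorative glowing jellyfish actor that bobs up and down with a tintable body and matching point light.
; Tick moves the mesh along local Z by Speed each frame, unscaled by delta time, flipping IfUp past plus or minus Lenth.
; The construction script creates dynamic materials for two mesh slots, sets Glow_Color from Color1 and copies it to the light.
; Diffuse_A is set twice, so Color2 overrides Color1.
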(event `self.ReceiveTick`
  (params (DeltaSeconds :type "Float (single-precision)"))
  (bind _sm_jellyfish0 (`self.SM_Jellyfish0`))
  (bind _lenth (`self.Lenth`))
  (bind _speed (`self.Speed`))
  (bind (_relativelocation_x _relativelocation_y _relativelocation_z) (`KismetMathLibrary.BreakVector` (`SceneComponent.RelativeLocation` _sm_jellyfish0)))
  (if (`self.ifUp`)
    (`SceneComponent.K2_AddLocalOffset` _sm_jellyfish0 (`KismetMathLibrary.MakeVector` 0.0 0.0 _speed) false false)
    (if (<= _relativelocation_z _lenth)
      (set `self.ifUp` true)
      (else
        (set `self.ifUp` false)))
    (else
      (`SceneComponent.K2_AddLocalOffset` _sm_jellyfish0 (`KismetMathLibrary.MakeVector` 0.0 0.0 (* _speed -1.0)) false false)
      (if (>= _relativelocation_z (* _lenth -1.0))
        (set `self.ifUp` false)
        (else
          (set `self.ifUp` true))))))

(fn `UserConstructionScript`
  (bind _sm_jellyfish0 (`self.SM_Jellyfish0`))
  (bind _color1 (`self.Color1`))
  (bind _returnvalue (`PrimitiveComponent.CreateDynamicMaterialInstance` _sm_jellyfish0 0 null "None"))
  (bind _returnvalue_2 (`PrimitiveComponent.CreateDynamicMaterialInstance` _sm_jellyfish0 1 null "None"))
  (`MaterialInstanceDynamic.SetVectorParameterValue` _returnvalue "Glow_Color" _color1)
  (`MaterialInstanceDynamic.SetVectorParameterValue` _returnvalue_2 "Glow_Color" _color1)
  (`MaterialInstanceDynamic.SetVectorParameterValue` _returnvalue "Diffuse_A" _color1)
  (`MaterialInstanceDynamic.SetVectorParameterValue` _returnvalue_2 "Diffuse_A" _color1)
  (`MaterialInstanceDynamic.SetVectorParameterValue` _returnvalue "Diffuse_A" (`self.Color2`))
  (`MaterialInstanceDynamic.SetVectorParameterValue` _returnvalue_2 "Diffuse_A" (`self.Color2`))
  (bind _returnvalue_3 (`MaterialInstanceDynamic.K2_GetVectorParameterValue` _returnvalue "Glow_Color"))
  (`LightComponent.SetLightColor` (`self.PointLight`) _returnvalue_3 true))