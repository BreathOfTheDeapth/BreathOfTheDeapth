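; Main tower that tracks how many light-guide towers are lit and drives progression to the Final level.
; OpenBuilding plays one of three Niagara sun animations chosen by Count, then a shared sound and expanding-ring burst that increments CompleteCount.
; Tick polls that counter: at two it reveals hidden tower actors and the shield and opens door collision.
; At three, material parameter collections drive an outline, then dissolve and blackout before the level loads.
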(event `self.ReceiveBeginPlay`
  ;[1 1 1] 主塔位置归零
  (`SkeletalMeshComponent.SetPosition` (`self.ANI_landmark`) 0.0 true))

(event `self.ReceiveTick`
  (params (DeltaSeconds :type "Float (single-precision)"))
  ;[1 1 1] 三座导光塔全部点亮
  (if (== (`self.Complete_Count`) 3)
    (`/Engine/EditorBlueprintResources/StandardMacros.DoOnce` false
      (:`Completed`
        ;[1 1 1] 描边后处理
        (bind (_direction `_新建轨道_0`) (`Timeline|时间轴_3`)
          (:`Update`
            (`KismetMaterialLibrary.SetScalarParameterValue` "/Game/JadeCiderquist/Material/Ocean/Scan/MPC_Scan.MPC_Scan" "RadiusStength" (`KismetMathLibrary.Lerp` 0.0 3.0 `_新建轨道_0`)))
          (:`Finished`
            (`|ExecutionSequence`
              (:`then_0`
                ;[1 1 1] 消散效果
                (bind (_direction_2 `_新建轨道_0_2`) (`Timeline|时间轴_6`)
                  (:`Update`
                    (`KismetMaterialLibrary.SetScalarParameterValue` "/Game/WengZhiBo/Material/All_Build.All_Build" "Strenth" (`KismetMathLibrary.Lerp` 0.0 1.0 `_新建轨道_0_2`)))))
              (:`then_1`
                ;[1 1 1] 黑场
                (bind (_direction_3 `_新建轨道_0_3`) (`Timeline|时间轴_4`)
                  (:`Update`
                    (`KismetMaterialLibrary.SetScalarParameterValue` "/Game/JadeCiderquist/Material/Underwater/MP_UnderWater.MP_UnderWater" "Light" (`KismetMathLibrary.Lerp` 1.0 0.0001 `_新建轨道_0_3`)))
                  (:`Finished`
                    (`GameplayStatics.OpenLevelBySoftObjectPtr` "/Game/Final.Final")))))))))
    (elif (== (`self.Complete_Count`) 2)
      (`/Engine/EditorBlueprintResources/StandardMacros.DoOnce` false
        (:`Completed`
          ;[1 1 1] 取消隐藏导光塔
          (bind _outactors (`GameplayStatics.GetAllActorsOfClassWithTag` "/Game/JadeCiderquist/BluePrint/BP_DaoGuangTa.BP_DaoGuangTa_C" "TA2"))
          (`self.SetActorHiddenInGame` _outactors false)
          (bind _outactors_2 (`GameplayStatics.GetAllActorsOfClass` "/Game/JadeCiderquist/BluePrint/BP_TaHand.BP_TaHand_C"))
          (`self.SetActorHiddenInGame` _outactors_2 false)
          ;[1 1 1] 保护罩显示
          (bind _outactors_3 (`GameplayStatics.GetAllActorsOfClass` "/Game/JadeCiderquist/Circle_Safe/BP_BaoHuZhao.BP_BaoHuZhao_C"))
          (bind _output (`|GetArrayItem` _outactors_3))
          (`PrimitiveComponent.SetCollisionEnabled` (`/Game/JadeCiderquist/Circle_Safe/BP_BaoHuZhao.qiuti_suiji` _output) "QueryAndPhysics")
          (`self.SetActorHiddenInGame` _output false)
          ;[1 1 1] 删除门碰撞
          (bind _outactors_4 (`GameplayStatics.GetAllActorsOfClass` "/Game/JadeCiderquist/BluePrint/BP_Door_Col.BP_Door_Col_C"))
          (bind _output_2 (`|GetArrayItem` _outactors_4))
          (bind _door_col (`/Game/JadeCiderquist/BluePrint/BP_Door_Col.Door_Col` _output_2))
          (`PrimitiveComponent.SetCollisionEnabled` _door_col "NoCollision")
          (`PrimitiveComponent.SetCollisionEnabled` (`/Game/JadeCiderquist/BluePrint/BP_Door_Col.Door_Col` (`|GetArrayItem` _outactors_4 1)) "NoCollision")
          (`SceneComponent.SetVisibility` _door_col false false)
          (`SceneComponent.SetVisibility` (`/Game/JadeCiderquist/BluePrint/BP_Door_Col.Door_Col` (`|GetArrayItem` _outactors_4 1)) false false)
          ;[1 1 1] 门引导
          (`SceneComponent.SetVisibility` (`/Game/JadeCiderquist/BluePrint/BP_Door_Col.SM_YinDaoQi` _output_2) true false))))))

(event `/Game/JadeCiderquist/BluePrint/BI_OpenBuilding.OpenBuilding`
  (bind _ns_sun (`self.NS_Sun`))
  (bind _ns_sun1 (`self.NS_Sun1`))
  (bind _ns_sun2 (`self.NS_Sun2`))
  ;[1 1 1] 点亮主塔逻辑
  (switch `int` (`self.Count`)
    (:`0`
      (bind (_direction `_新建轨道_0`) (`Timeline|时间轴_0` :!via `PlayFromStart`)
        (:`Update`
          (`SceneComponent.SetRelativeScale3D` _ns_sun (`KismetMathLibrary.Conv_DoubleToVector` (`KismetMathLibrary.Lerp` 40.0 1.0 `_新建轨道_0`)))
          (`FXSystemComponent.SetFloatParameter` _ns_sun "Drag" (`KismetMathLibrary.Lerp` 2000.0 160.0 `_新建轨道_0`)))
        (:`Finished`
          (`GameplayStatics.PlaySound2D` "/Game/JadeCiderquist/Sound/MainBuilding_lightup.MainBuilding_lightup" 1.0 1.0 0.0 null null :!label _label)
          (bind (_direction_2 `_新建轨道_0_2`) (`Timeline|时间轴_5` :!via `PlayFromStart`)
            (:`Update`
              (`SceneComponent.SetRelativeScale3D` (`self.Ring`) (`KismetMathLibrary.Conv_DoubleToVector` (`KismetMathLibrary.Lerp` 0.0 5000.0 `_新建轨道_0_2`)))
              (`SceneComponent.SetRelativeScale3D` (`self.Ring1`) (`KismetMathLibrary.Conv_DoubleToVector` (`KismetMathLibrary.Lerp` 0.0 2000.0 `_新建轨道_0_2`))))
            (:`Finished`
              (bind _output_get (set `self.Complete_Count` (+ (stale _output_get) 1)))
              (`SceneComponent.SetRelativeScale3D` (`self.Ring`) (0.0 0.0 0.0))
              (`SceneComponent.SetRelativeScale3D` (`self.Ring1`) (0.0 0.0 0.0)))))))
    (:`1`
      (bind (_direction_3 `_新建轨道_0_3`) (`Timeline|时间轴_1` :!via `PlayFromStart`)
        (:`Update`
          (`SceneComponent.SetRelativeScale3D` _ns_sun1 (`KismetMathLibrary.Conv_DoubleToVector` (`KismetMathLibrary.Lerp` 40.0 1.0 `_新建轨道_0_3`)))
          (`FXSystemComponent.SetFloatParameter` _ns_sun1 "Drag" (`KismetMathLibrary.Lerp` 2000.0 160.0 `_新建轨道_0_3`)))
        (:`Finished`
          (goto _label))))
    (:`2`
      (bind (_direction_4 `_新建轨道_0_4`) (`Timeline|时间轴_2` :!via `PlayFromStart`)
        (:`Update`
          (`SceneComponent.SetRelativeScale3D` _ns_sun2 (`KismetMathLibrary.Conv_DoubleToVector` (`KismetMathLibrary.Lerp` 40.0 1.0 `_新建轨道_0_4`)))
          (`FXSystemComponent.SetFloatParameter` _ns_sun2 "Drag" (`KismetMathLibrary.Lerp` 2000.0 160.0 `_新建轨道_0_4`)))
        (:`Finished`
          (goto _label))))))

(fn `UserConstructionScript`)