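; Boss vortex actor that teleports the VR player on contact, noted as to the third light-guide tower.
; BeginPlay tints the Niagara vortex with its Color variable.
; Sphere overlap locks pawn movement and fades the Light parameter in MP_UnderWater to black, then a timeline finish restores movement, moves the first found pawn to NewLocation and fades back in.
; A vortex-appearance alpha timeline exists but is never triggered.
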(event `self.ReceiveBeginPlay`
  (`NiagaraComponent.SetVariableLinearColor` (`self.NS_Vortex_Boss`) "XW_Color" (`self.Color`)))

(event `self.Sphere.OnComponentBeginOverlap`
  (params (OverlappedComponent :type "PrimitiveComponent Object Reference") (OtherActor :type "Actor Object Reference") (OtherComp :type "PrimitiveComponent Object Reference") (OtherBodyIndex :type Integer) (bFromSweep :type Boolean) (SweepResult :type "HitResult Structure (by ref)"))
  (bind _asbp_pawn_vr_char_example_hands_on (cast `/Game/AFCore/Examples/Pawns/VR/BP_Pawn_VR_Char_Example_HandsOn` OtherActor))
  (set `/Game/AFCore/Examples/Pawns/VR/BP_Pawn_VR_Char_Example_HandsOn.if_Move` false _asbp_pawn_vr_char_example_hands_on)
  (bind (_direction `_新建轨道_0`) (`Timeline|时间轴_1`)
    (:`Update`
      (`KismetMaterialLibrary.SetScalarParameterValue` "/Game/JadeCiderquist/Material/Underwater/MP_UnderWater.MP_UnderWater" "Light" (`KismetMathLibrary.Lerp` 1.0 0.0 `_新建轨道_0`)))
    (:`Finished`
      (bind _outactors (`GameplayStatics.GetAllActorsOfClass` "/Game/AFCore/Examples/Pawns/VR/BP_Pawn_VR_Char_Example_HandsOn.BP_Pawn_VR_Char_Example_HandsOn_C"))
      (set `/Game/AFCore/Examples/Pawns/VR/BP_Pawn_VR_Char_Example_HandsOn.if_Move` true (`|GetArrayItem` _outactors))
      ;[1 1 1] 瞬移至第三座导光塔
      (bind _outactors_2 (`GameplayStatics.GetAllActorsOfClass` "/Game/AFCore/Examples/Pawns/VR/BP_Pawn_VR_Char_Example_HandsOn.BP_Pawn_VR_Char_Example_HandsOn_C"))
      (`self.K2_SetActorLocation` (`|GetArrayItem` _outactors_2) (`self.New Location`) false false)
      ;[1 1 1] 黑场变亮
      (bind (_direction_2 `_新建轨道_0_2`) (`Timeline|时间轴_2` :!via `PlayFromStart`)
        (:`Update`
          (`KismetMaterialLibrary.SetScalarParameterValue` "/Game/JadeCiderquist/Material/Underwater/MP_UnderWater.MP_UnderWater" "Light" (`KismetMathLibrary.Lerp` 0.0 1.0 `_新建轨道_0_2`)))))))

(fn `UserConstructionScript`)