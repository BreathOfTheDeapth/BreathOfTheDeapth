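; BP_TaHand is a VR hand scanner that powers a light-guide tower when latched by a left hand with three collected fires.
; A completed scan timeline consumes those fires, lights the tagged BP_DaoGuangTa line, saves the player's relocation point and fires the matching BP_GuangShu beam.
; HandCount selects the tower and is passed to BP_MainBuilding; the second tower gates that signal until complete or ComTA is called.
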(event `self.ReceiveBeginPlay`
  (bind _returnvalue (`PrimitiveComponent.CreateDynamicMaterialInstance` (`self.SM_Handscanner`) 1 "/Game/WengZhiBo/Material/M_Fire.M_Fire" "None"))
  (set `self.DynMaterial` _returnvalue))

(event `self.Comp_Latch.Latch_ActorGotLatched`
  (params (LatchingPawn :type "/Game/AFCore/Blueprints/Pawn/BP_Pawn_Base Object Reference") (LatchingActor :type "Actor Object Reference"))
  (bind _hand_count (`self.Hand_Count`))
  (bind _asbp_mcomp (cast `/Game/AFCore/Blueprints/VR/MotionComponents/BP_MComp` LatchingActor))
  (`SceneComponent.SetVisibility` (`self.SM_YinDaoQi`) false false)
  (`MaterialInstanceDynamic.SetVectorParameterValue` (`self.DynMaterial`) "color" (struct :`G` 0.794128 :`B` 2.0 :`A` 1.0))
  (bind _outactors (`GameplayStatics.GetAllActorsOfClass` "/Game/AFCore/Examples/Pawns/VR/BP_Pawn_VR_Char_Example_HandsOn.BP_Pawn_VR_Char_Example_HandsOn_C"))
  (bind _output (`|GetArrayItem` _outactors))
  (if (>= (`/Game/AFCore/Examples/Pawns/VR/BP_Pawn_VR_Char_Example_HandsOn.Fire_Count` _output) 3)
    (switch `/Game/AFCore/Enums/Enum_Side` (`/Game/AFCore/Blueprints/VR/MotionComponents/BP_MComp.Side` _asbp_mcomp)
      (:`NewEnumerator0`
        (`SceneComponent.SetVisibility` (`self.Decal`) true false)
        (bind (_direction _lerp) (`Timeline|LatchTimeline` :!label _label)
          (:`Update`
            (`SceneComponent.K2_SetRelativeLocation` (`self.DecalOffset`) (`KismetMathLibrary.MakeVector` 0.0 0.0 (`KismetMathLibrary.Lerp` 0.0 -18.0 _lerp)) false false))
          (:`Finished`
            ;[1 1 1] 成功
            (`SceneComponent.SetVisibility` (`self.Decal`) false false)
            (switch `ETimelineDirection` _direction
              (:`Forward`
                (`MaterialInstanceDynamic.SetVectorParameterValue` (`self.DynMaterial`) "color" (struct :`G` 5.722922 :`B` 15.0 :`A` 1.0))
                (if (== (`self.Hand_Count`) 0)
                  ;[1 1 1] 主建筑动画
                  (bind _outactors_2 (`GameplayStatics.GetAllActorsOfClass` "/Game/JadeCiderquist/BluePrint/BP_MainBuilding.BP_MainBuilding_C"))
                  (`SkeletalMeshComponent.Play` (`/Game/JadeCiderquist/BluePrint/BP_MainBuilding.ANI_landmark` (`|GetArrayItem` _outactors_2)) false))
                ;[1 1 1] 删除3个火焰
                (for _ (range 3)
                  (bind _outactors_3 (`GameplayStatics.GetAllActorsOfClass` "/Game/AFCore/Examples/Pawns/VR/BP_Pawn_VR_Char_Example_HandsOn.BP_Pawn_VR_Char_Example_HandsOn_C"))
                  (bind _bp_fire (`/Game/AFCore/Examples/Pawns/VR/BP_Pawn_VR_Char_Example_HandsOn.BP_Fire` (`|GetArrayItem` _outactors_3)))
                  (bind _output_2 (`|GetArrayItem` _bp_fire (- (`KismetArrayLibrary.Array_Length` _bp_fire) 1)))
                  (`self.K2_DestroyActor` _output_2)
                  (`KismetArrayLibrary.Array_RemoveItem` _bp_fire _output_2)
                  ;[1 1 1] 线条发光
                  (bind _outactors_4 (`GameplayStatics.GetAllActorsOfClassWithTag` "/Game/JadeCiderquist/BluePrint/BP_DaoGuangTa.BP_DaoGuangTa_C" (`|GetArrayItem` (`self.Tag`) (`self.Hand_Count`))))
                  (bind _output_3 (`|GetArrayItem` _outactors_4))
                  (bind _returnvalue (`PrimitiveComponent.CreateDynamicMaterialInstance` (`/Game/JadeCiderquist/BluePrint/BP_DaoGuangTa.M_LightC` _output_3) 0 "/Game/JadeCiderquist/Material/Light_Ta_Red.Light_Ta_Red" "None"))
                  (`MaterialInstanceDynamic.SetScalarParameterValue` _returnvalue "Alpha" 0.0)
                  (bind _returnvalue_2 (`PrimitiveComponent.CreateDynamicMaterialInstance` (`/Game/JadeCiderquist/BluePrint/BP_DaoGuangTa.MechanismA_Mechanism05_F` _output_3) 0 "/Game/JadeCiderquist/Material/M_Line_Color.M_Line_Color" "None"))
                  (bind (_direction_2 `_新建轨道_0`) (`Timeline|时间轴_0`)
                    (:`Update`
                      (`MaterialInstanceDynamic.SetScalarParameterValue` _returnvalue_2 "Pos" (`KismetMathLibrary.Lerp` 0.0 3.0 `_新建轨道_0`))
                      (`/Engine/EditorBlueprintResources/StandardMacros.DoOnce` false
                        (:`Completed`
                          (`KismetSystemLibrary.Delay` 1.0)
                          (bind _audio (`/Game/JadeCiderquist/BluePrint/BP_DaoGuangTa.Audio` _output_3))
                          (`AudioComponent.Play` _audio 0.0))))
                    (:`Finished`
                      (`AudioComponent.Stop` _audio)
                      ;[1 1 1] 导光塔存档点
                      (bind _outactors_5 (`GameplayStatics.GetAllActorsOfClass` "/Game/AFCore/Examples/Pawns/VR/BP_Pawn_VR_Char_Example_HandsOn.BP_Pawn_VR_Char_Example_HandsOn_C"))
                      (bind _output_4 (`|GetArrayItem` _outactors_5))
                      (set `/Game/AFCore/Examples/Pawns/VR/BP_Pawn_VR_Char_Example_HandsOn.PlayerRe_Location` (`self.K2_GetActorLocation` _output_4) _output_4)
                      ;[1 1 1] 光束发射
                      (bind _outactors_6 (`GameplayStatics.GetAllActorsOfClassWithTag` "/Game/JadeCiderquist/BluePrint/BP_GuangShu.BP_GuangShu_C" (`|GetArrayItem` (`self.Tag`) (`self.Hand_Count`))))
                      (bind _output_5 (`|GetArrayItem` _outactors_6))
                      (`ActorComponent.Activate` (`/Game/JadeCiderquist/BluePrint/BP_GuangShu.NS_LightTa` _output_5) false)
                      (bind _returnvalue_3 (`PrimitiveComponent.CreateDynamicMaterialInstance` (`/Game/JadeCiderquist/BluePrint/BP_GuangShu.M_LightC` _output_5) 0 "/Game/JadeCiderquist/Material/Light_Ta_Inst.Light_Ta_Inst" "None"))
                      (`MaterialInstanceDynamic.SetScalarParameterValue` _returnvalue_3 "Alpha" 5.0)
                      (`AudioComponent.Play` (`/Game/JadeCiderquist/BluePrint/BP_GuangShu.Audio` _output_5) 0.0)
                      (bind (_direction_3 `_新建轨道_0_2`) (`Timeline|时间轴_1`)
                        (:`Update`
                          (`MaterialInstanceDynamic.SetScalarParameterValue` _returnvalue_3 "Top" (`KismetMathLibrary.Lerp` 100.0 0.3 `_新建轨道_0_2`)))
                        (:`Finished`
                          ;[1 1 1] 判断是否是第二座塔（需要旋转）
                          (if (not (!= _hand_count 1))
                            (bind _outactors_7 (`GameplayStatics.GetAllActorsOfClass` "/Game/JadeCiderquist/BluePrint/BP_DaoGuangTa.BP_DaoGuangTa_C"))
                            (if (`/Game/JadeCiderquist/BluePrint/BP_DaoGuangTa.Complete` (`|GetArrayItem` _outactors_7 _hand_count))
                              _
                              (else
                                (goto _label_4 :!via `Open`))))
                          ;[1 1 1] 主塔播放特效信号
                          (bind _outactors_8 (`GameplayStatics.GetAllActorsOfClass` "/Game/JadeCiderquist/BluePrint/BP_MainBuilding.BP_MainBuilding_C" :!label _label_2))
                          (bind _output_6 (`|GetArrayItem` _outactors_8))
                          (set `/Game/JadeCiderquist/BluePrint/BP_MainBuilding.Count` (`self.Hand_Count`) _output_6)
                          (message `/Game/JadeCiderquist/BluePrint/BI_OpenBuilding.OpenBuilding` _output_6))))))
                (bind _output_get (set `/Game/AFCore/Examples/Pawns/VR/BP_Pawn_VR_Char_Example_HandsOn.Fire_Count` (- (stale _output_get) 3) _output)))))))
      (:`NewEnumerator1`
        (`MaterialInstanceDynamic.SetVectorParameterValue` (`self.DynMaterial`) "color" (struct :`G` 0.115486 :`B` 0.255208 :`A` 1.0) :!label _label_3)))
    (else
      (goto _label_3))))

(event `self.Comp_Latch.Latch_ActorLatchReleased`
  (params (ReleasingPawn :type "/Game/AFCore/Blueprints/Pawn/BP_Pawn_Base Object Reference") (ReleasingActor :type "Actor Object Reference"))
  (goto _label :!via `Reverse`))

(event `/Game/JadeCiderquist/BluePrint/BI_OpenBuilding.Com_TA`
  (`/Engine/EditorBlueprintResources/StandardMacros.DoOnce` false
    (:`Completed`
      (`/Engine/EditorBlueprintResources/StandardMacros.Gate` true :!label _label_4
        (:`Exit`
          (goto _label_2))))))

(fn `UserConstructionScript`
  (`SceneComponent.SetVisibility` (`self.SM_YinDaoQi`) (`self.引导`) false))