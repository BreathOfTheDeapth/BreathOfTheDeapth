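; VR pistol actor that is picked up through a grab component and fires projectiles from its muzzle on trigger, with sound, haptics and an ammo count.
; An empty magazine plays a dry-fire sound and shows the pawn's no-ammo widget once; the reload logic is unconnected.
; Grab and release toggle the pawn's shark-detection sphere collision.
; Once picked up, a dropped gun returns to the right controller via a delayed Tick timeline lerp and a release-timer teleport.
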(event `self.ReceiveTick`
  (params (DeltaSeconds :type "Float (single-precision)"))
  ;[1 1 1] 检测玩家有没有丢枪，丢枪后瞬移过去
  (`KismetSystemLibrary.Delay` 1.0)
  (if (`self.Pick_Once`)
    (if (not (`self.Pick_Up`))
      (bind _outactors (`GameplayStatics.GetAllActorsOfClass` "/Game/AFCore/Examples/Pawns/VR/BP_Pawn_VR_Char_Example_HandsOn.BP_Pawn_VR_Char_Example_HandsOn_C"))
      (set `self.Now_Location` (`self.K2_GetActorLocation`))
      (bind (_direction `_新建轨道_0`) (`Timeline|时间轴_0` :!via `PlayFromStart`)
        (:`Update`
          (`self.K2_SetActorLocation` (`KismetMathLibrary.VLerp` (`self.Now_Location`) (`SceneComponent.K2_GetComponentLocation` (`/Game/AFCore/Blueprints/Pawn/VR/BP_Pawn_VR.MotionControllerRight` (`|GetArrayItem` _outactors))) `_新建轨道_0`)))))))

(event `self.Comp_Grab.Grab_ActorPickedUp`
  (params (GrabbingPawn :type "/Game/AFCore/Blueprints/Pawn/BP_Pawn_Base Object Reference") (GrabbingActor :type "Actor Object Reference"))
  ;[1 1 1] 拾取枪支
  (`SceneComponent.SetVisibility` (`self.SM_YinDaoQi`) false false)
  (set `self.Pick_Once` true)
  (set `self.Pick_Up` true)
  ;[1 1 1] 拾取枪，开启鲨鱼检测碰撞
  (bind _outactors (`GameplayStatics.GetAllActorsOfClass` "/Game/AFCore/Examples/Pawns/VR/BP_Pawn_VR_Char_Example_HandsOn.BP_Pawn_VR_Char_Example_HandsOn_C"))
  (`PrimitiveComponent.SetCollisionEnabled` (`/Game/AFCore/Examples/Pawns/VR/BP_Pawn_VR_Char_Example_HandsOn.Sharke_Sphere` (`|GetArrayItem` _outactors)) "QueryAndPhysics"))

(event `self.Comp_Grab.Grab_ActorReleased`
  (params (ReleasingPawn :type "/Game/AFCore/Blueprints/Pawn/BP_Pawn_Base Object Reference") (ReleasingActor :type "Actor Object Reference") (LastRelease :type Boolean))
  (set `self.Pick_Up` false)
  (`|ExecutionSequence`
    (:`then_0`
      (`KismetSystemLibrary.Delay` 4.0)
      (if (not (`self.Pick_Up`))
        ;[1 1 1] 松开手枪后自动设置到右手
        (bind _outactors (`GameplayStatics.GetAllActorsOfClass` "/Game/AFCore/Examples/Pawns/VR/BP_Pawn_VR_Char_Example_HandsOn.BP_Pawn_VR_Char_Example_HandsOn_C"))
        (`self.K2_SetActorLocation` (`SceneComponent.K2_GetComponentLocation` (`/Game/AFCore/Blueprints/Pawn/VR/BP_Pawn_VR.MotionControllerRight` (`|GetArrayItem` _outactors))))))
    (:`then_1`
      ;[1 1 1] 丢枪，关闭鲨鱼检测碰撞
      (bind _outactors_2 (`GameplayStatics.GetAllActorsOfClass` "/Game/AFCore/Examples/Pawns/VR/BP_Pawn_VR_Char_Example_HandsOn.BP_Pawn_VR_Char_Example_HandsOn_C"))
      (`PrimitiveComponent.SetCollisionEnabled` (`/Game/AFCore/Examples/Pawns/VR/BP_Pawn_VR_Char_Example_HandsOn.Sharke_Sphere` (`|GetArrayItem` _outactors_2)) "NoCollision"))))

(event `self.ReceiveBeginPlay`)

(event `self.Comp_Grab.Grab_KeyInput`
  (params (MComp :type "/Game/AFCore/Blueprints/VR/MotionComponents/BP_MComp Object Reference") (Key :type "/Game/AFCore/Enums/Enum_Controller_Buttons Enum" :default "NewEnumerator1") (Set :type Boolean))
  (bind _returnvalue (`GameplayStatics.GetPlayerController` 0))
  (bind _pistolfirehapticeffect (`self.PistolFireHapticEffect`))
  (bind _fx_shot (`self.Fx_Shot`))
  (bind _muzzlelocation (`self.MuzzleLocation`))
  (switch `/Game/AFCore/Enums/Enum_Controller_Buttons` Key
    (:`NewEnumerator0`
      (if Set
        (if (> (`self.ZD_Count`) 0)
          (`ActorComponent.Deactivate` _fx_shot)
          (`ActorComponent.Activate` _fx_shot false)
          ;[1 1 1] 开枪减子弹数
          (bind _output_get (set `self.ZD_Count` (- (stale _output_get) 1)))
          (`GameplayStatics.PlaySound2D` "/Game/JadeCiderquist/Sound/Gun_Shot.Gun_Shot" 1.0 1.0 0.0 null null)
          (switch `/Game/AFCore/Enums/Enum_Side` (`/Game/AFCore/Blueprints/VR/MotionComponents/BP_MComp.Side` MComp)
            (:`NewEnumerator0`
              (`PlayerController.PlayHapticEffect` _returnvalue _pistolfirehapticeffect "Left" 1.0 false))
            (:`NewEnumerator1`
              (`PlayerController.PlayHapticEffect` _returnvalue _pistolfirehapticeffect "Right" 1.0 false)))
          ;[1 1 1] 生成子弹
          (`|SpawnActorFromClass` "/Game/JadeCiderquist/Gun/Blueprints/Projectile.Projectile_C" (`KismetMathLibrary.MakeTransform` (`SceneComponent.K2_GetComponentLocation` _muzzlelocation) (`SceneComponent.K2_GetComponentRotation` _muzzlelocation)) "Undefined" "OverrideRootScale" self (`GameplayStatics.GetPlayerPawn` 0))
          (else
            ;[1 1 1] 没子弹了
            (`GameplayStatics.PlaySound2D` "/Game/JadeCiderquist/Sound/Gun_NoShot.Gun_NoShot" 1.0 1.0 0.0 null null)
            (`/Engine/EditorBlueprintResources/StandardMacros.DoOnce` false
              (:`Completed`
                (bind _outactors (`GameplayStatics.GetAllActorsOfClass` "/Game/AFCore/Examples/Pawns/VR/BP_Pawn_VR_Char_Example_HandsOn.BP_Pawn_VR_Char_Example_HandsOn_C"))
                (`SceneComponent.SetVisibility` (`/Game/AFCore/Examples/Pawns/VR/BP_Pawn_VR_Char_Example_HandsOn.WBP_NoShot` (`|GetArrayItem` _outactors)) true false)))))))))

(fn `UserConstructionScript`)