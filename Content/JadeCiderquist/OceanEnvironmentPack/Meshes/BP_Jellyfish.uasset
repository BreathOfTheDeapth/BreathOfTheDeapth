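; Decorative jellyfish actor that bobs vertically and casts light matching its material's glow color.
; The construction script assigns both mesh materials, creating a dynamic instance for the first and copying its Glow_Color to the point light.
; Tick moves the mesh along local Z by Speed, flipping direction when relative height passes positive or negative Lenth.
; The step is not scaled by delta time, so bob speed depends on frame rate.
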(event `self.ReceiveTick`
  (params (DeltaSeconds :type "Float (single-precision)"))
  (bind _sm_jellyfish0 (`self.SM_Jellyfish0`))
  (bind _lenth (`self.Lenth`))
  (bind _speed (`self.Speed`))
  (bind (_relativelocation_x _relativelocation_y _relativelocation_z) (`KismetMathLibrary.BreakVector` (`SceneComponent.RelativeLocation` _sm_jellyfish0)))
  (if (`self.ifUp`)
    (`SceneComponent.K2_AddLocalOffset` _sm_jellyfish0 (`KismetMathLibrary.MakeVector` 0.0 0.0 _speed) false false)
    (if (<= _relativelocation_z _lenth)
      (set `self.ifUp` true)
      (else
        (set `self.ifUp` false)))
    (else
      (`SceneComponent.K2_AddLocalOffset` _sm_jellyfish0 (`KismetMathLibrary.MakeVector` 0.0 0.0 (* _speed -1.0)) false false)
      (if (>= _relativelocation_z (* _lenth -1.0))
        (set `self.ifUp` false)
        (else
          (set `self.ifUp` true))))))

(fn `UserConstructionScript`
  (bind _sm_jellyfish0 (`self.SM_Jellyfish0`))
  (bind _returnvalue (`PrimitiveComponent.CreateDynamicMaterialInstance` _sm_jellyfish0 0 (`self.Material1`) "None"))
  (bind _returnvalue_2 (`MaterialInstanceDynamic.K2_GetVectorParameterValue` _returnvalue "Glow_Color"))
  (`LightComponent.SetLightColor` (`self.PointLight`) _returnvalue_2 true)
  (`PrimitiveComponent.SetMaterial` _sm_jellyfish0 0 _returnvalue)
  (`PrimitiveComponent.SetMaterial` _sm_jellyfish0 1 (`self.Material2`)))