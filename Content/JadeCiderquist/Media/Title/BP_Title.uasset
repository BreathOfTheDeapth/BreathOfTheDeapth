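; BP_Title is a title-sequence actor that plays a media title on a plane, shows three texts, then destroys itself.
; BeginPlay primes the media paused; once PlayTitle is set, Tick plays it once, then raises M_Title's "Strenth" parameter through a dynamic material.
; Timelines, chained by Delays on their Update pins, fade each text in and out.
; Before Text3, it sends ComXuanWoMessage to BP_Xuanwo vortex actors.
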(event `self.ReceiveBeginPlay`
  (bind _media (`self.Media`))
  ;[1 1 1] 重置标题
  (`MediaPlayer.OpenSource` _media "/Game/JadeCiderquist/Media/Title/Sourse_Title.Sourse_Title")
  (`KismetSystemLibrary.Delay` 0.01)
  (`MediaPlayer.Rewind` _media)
  (`MediaPlayer.Pause` _media))

(event `self.ReceiveTick`
  (params (DeltaSeconds :type "Float (single-precision)"))
  (bind _media (`self.Media`))
  (if (`self.Play_Title`)
    (`/Engine/EditorBlueprintResources/StandardMacros.DoOnce` false
      (:`Completed`
        (`KismetSystemLibrary.Delay` 1.0)
        ;[1 1 1] 播放标题
        (`MediaPlayer.Play` _media)
        (`KismetSystemLibrary.Delay` 4.5)
        (`MediaPlayer.Pause` _media)
        (`KismetSystemLibrary.Delay` 1.0)
        ;[1 1 1] 标题结束
        (bind (_direction `_新建轨道_0`) (`Timeline|时间轴_0`)
          (:`Update`
            (`MaterialInstanceDynamic.SetScalarParameterValue` (`self.Material`) "Strenth" (`KismetMathLibrary.Lerp` 0.0 1.0 `_新建轨道_0`))
            (`KismetSystemLibrary.Delay` 2.0)
            ;[1 1 1] Text1
            (bind (_direction_2 `_新建轨道_0_2`) (`Timeline|时间轴_1`)
              (:`Update`
                (`WidgetComponent.SetTintColorAndOpacity` (`self.Text1`) (make `LinearColor` 1.0 1.0 1.0 (`KismetMathLibrary.Lerp` 0.0 0.3 `_新建轨道_0_2`)))
                (`KismetSystemLibrary.Delay` (`self.Text_Time`))
                (bind (_direction_3 `_新建轨道_0_3`) (`Timeline|时间轴_2`)
                  (:`Update`
                    (`WidgetComponent.SetTintColorAndOpacity` (`self.Text1`) (make `LinearColor` 1.0 1.0 1.0 (`KismetMathLibrary.Lerp` 0.3 0.0 `_新建轨道_0_3`)))
                    (`KismetSystemLibrary.Delay` (`self.Text_Time`))
                    ;[1 1 1] Text2
                    (bind (_direction_4 `_新建轨道_0_4`) (`Timeline|时间轴_3`)
                      (:`Update`
                        (`WidgetComponent.SetTintColorAndOpacity` (`self.Text2`) (make `LinearColor` 1.0 1.0 1.0 (`KismetMathLibrary.Lerp` 0.0 0.3 `_新建轨道_0_4`)))
                        (`KismetSystemLibrary.Delay` (`self.Text_Time`))
                        (bind (_direction_5 `_新建轨道_0_5`) (`Timeline|时间轴_4`)
                          (:`Update`
                            (`WidgetComponent.SetTintColorAndOpacity` (`self.Text2`) (make `LinearColor` 1.0 1.0 1.0 (`KismetMathLibrary.Lerp` 0.3 0.0 `_新建轨道_0_5`)))
                            (`KismetSystemLibrary.Delay` (`self.Text_Time`))
                            ;[1 1 1] 漩涡
                            (bind _outactors (`GameplayStatics.GetAllActorsOfClass` "/Game/JadeCiderquist/BluePrint/BP_Xuanwo.BP_Xuanwo_C"))
                            (message `/Game/JadeCiderquist/BluePrint/BI_XuanWo.Com_XuanWo` _outactors)
                            ;[1 1 1] Text3
                            (bind (_direction_6 `_新建轨道_0_6`) (`Timeline|时间轴_5`)
                              (:`Update`
                                (`WidgetComponent.SetTintColorAndOpacity` (`self.Text3`) (make `LinearColor` 1.0 1.0 1.0 (`KismetMathLibrary.Lerp` 0.0 0.3 `_新建轨道_0_6`)))
                                (`KismetSystemLibrary.Delay` (`self.Text_Time`))
                                (bind (_direction_7 `_新建轨道_0_7`) (`Timeline|时间轴_6`)
                                  (:`Update`
                                    (`WidgetComponent.SetTintColorAndOpacity` (`self.Text3`) (make `LinearColor` 1.0 1.0 1.0 (`KismetMathLibrary.Lerp` 0.3 0.0 `_新建轨道_0_7`)))
                                    (`KismetSystemLibrary.Delay` (`self.Text_Time`))
                                    (`self.K2_DestroyActor`)))))))))))))))))))

(fn `UserConstructionScript`
  (bind _returnvalue (`PrimitiveComponent.CreateDynamicMaterialInstance` (`self.Plane`) 0 "/Game/JadeCiderquist/Media/Title/M_Title.M_Title" "None"))
  (set `self.Material` _returnvalue))